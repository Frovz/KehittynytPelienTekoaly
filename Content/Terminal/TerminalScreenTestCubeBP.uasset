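; Test actor for a terminal screen that draws lines of text onto a cube's material at runtime.
; On BeginPlay it creates a canvas render target and feeds it as a texture parameter into a dynamic material instance on the static mesh.
; The render target's update event draws each TerminalText entry as a stacked line.
; A one-shot timer later swaps in hardcoded Finnish test strings and calls UpdateResource to redraw.
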(event `RenderTextEvent`
  (params (Canvas :type "Canvas Object Reference") (Width :type Integer) (Height :type Integer))
  (for (_array_element _array_index) (`self.Terminal Text`)
    (`Canvas.K2_DrawText` Canvas "/Engine/EngineFonts/Roboto.Roboto" _array_element (`KismetMathLibrary.MakeVector2D` 100.0 (+ (* _array_index 100.0) 100.0)) (2.0 2.0) (struct :`R` 1.0 :`G` 1.0 :`B` 1.0 :`A` 1.0) 0.0 (struct :`A` 1.0) (1.0 1.0) false false false (struct :`A` 1.0))))

(event `self.ReceiveBeginPlay`
  (`|ExecutionSequence`
    (:`then_0`
      (bind _returnvalue (`CanvasRenderTarget2D.CreateCanvasRenderTarget2D` "/Game/Terminal/TerminalCanvasRenderTargetBP.TerminalCanvasRenderTargetBP_C"))
      (bind _output_get (set `self.ScreenText` _returnvalue))
      (add `CanvasRenderTarget2D.OnCanvasRenderTargetUpdate` _output_get (delegate `RenderTextEvent`))
      (`CanvasRenderTarget2D.UpdateResource` (`self.ScreenText`)))
    (:`then_1`
      (bind _returnvalue_2 (`KismetMaterialLibrary.CreateDynamicMaterialInstance` "/Game/Terminal/TerminalScreenTestCubeMaterial.TerminalScreenTestCubeMaterial"))
      (`PrimitiveComponent.SetMaterial` (`self.StaticMeshComponent`) 0 _returnvalue_2)
      (`MaterialInstanceDynamic.SetTextureParameterValue` _returnvalue_2 "ScreenTextureTest" (`self.ScreenText`)))
    (:`then_2`
      (`KismetSystemLibrary.K2_SetTimerDelegate` (delegate `ChangeText`) 5.0))))

(event `ChangeText`
  (set `self.Terminal Text` (`|MakeArray` "Nyt" "Se" "Teksti" "Vaihtui"))
  (`CanvasRenderTarget2D.UpdateResource` (`self.ScreenText`)))

(fn `UserConstructionScript`)