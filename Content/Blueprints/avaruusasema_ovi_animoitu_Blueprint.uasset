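; Animated space station door that opens and closes as a Player-tagged actor enters or leaves its trigger box.
; Box overlaps play the open or close animation on the skeletal mesh.
; Tick and both overlap handlers sync the Sparks ribbon emitters to whether that animation is playing.
; A looping timer resets the play rate through a random range whose equal bounds make it a constant half speed.
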(event `self.ReceiveBeginPlay`
  (`|ExecutionSequence`
    (:`then_0`
      (`FXSystemComponent.SetEmitterEnable` (`self.Sparks`) "RibbonSource" false)
      (`FXSystemComponent.SetEmitterEnable` (`self.Sparks`) "Ribbon" false))
    (:`then_1`
      (`KismetSystemLibrary.K2_SetTimer` null "PlayRateChange" 0.5 true))))

(event `self.ReceiveTick`
  (params (DeltaSeconds :type "Float (single-precision)"))
  (bind _returnvalue (`SkeletalMeshComponent.IsPlaying` (`self.SkeletalMeshComponent`)))
  (`FXSystemComponent.SetEmitterEnable` (`self.Sparks`) "RibbonSource" _returnvalue :!label _label)
  (`FXSystemComponent.SetEmitterEnable` (`self.Sparks`) "Ribbon" _returnvalue))

(event `self.Box.OnComponentBeginOverlap`
  (params (OverlappedComponent :type "PrimitiveComponent Object Reference") (OtherActor :type "Actor Object Reference") (OtherComp :type "PrimitiveComponent Object Reference") (OtherBodyIndex :type Integer) (bFromSweep :type Boolean) (SweepResult :type "HitResult Structure (by ref)"))
  (if (`self.ActorHasTag` OtherActor "Player")
    (`self.OpenDoor`)
    (goto _label)))

(event `self.Box.OnComponentEndOverlap`
  (params (OverlappedComponent :type "PrimitiveComponent Object Reference") (OtherActor :type "Actor Object Reference") (OtherComp :type "PrimitiveComponent Object Reference") (OtherBodyIndex :type Integer))
  (if (`self.ActorHasTag` OtherActor "Player")
    (`self.CloseDoor`)
    (goto _label)))

(fn `CloseDoor`
  (`SkeletalMeshComponent.PlayAnimation` (`self.SkeletalMeshComponent`) "/Game/Station/avaruusasema_ovi_animoitu_Anim_Close.avaruusasema_ovi_animoitu_Anim_Close" false))

(fn `OpenDoor`
  (`SkeletalMeshComponent.PlayAnimation` (`self.SkeletalMeshComponent`) "/Game/Station/avaruusasema_ovi_animoitu_Anim_Open.avaruusasema_ovi_animoitu_Anim_Open" false))

(fn `PlayRateChange`
  (`SkeletalMeshComponent.SetPlayRate` (`self.SkeletalMeshComponent`) (`KismetMathLibrary.RandomFloatInRange` 0.5 0.5)))

(fn `UserConstructionScript`)